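; Main player controller that sets up input and starts the game through GM_MainGameMode.
; On BeginPlay it adds the MC_Viewer Enhanced Input mapping context, caches the game mode and calls InitialiseGame with the owning controller.
; Hard-coded test keys cycle the selected example player left and right with wraparound, toggle player icons, and start a raffle, all delegated to the game mode.
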(event EventBeginPlay
  (bind _self self)
  (bind _returnvalue (PlayerController|LocalPlayerSubsystems|GetEnhancedInputLocalPlayerSubsystem _self))
  ;[1 1 1] Sets up player inputs
  (Utilities|IsValid _returnvalue
    (:Is%20Valid
      (Input|AddMappingContext _returnvalue "/Game/Input/MC_Viewer.MC_Viewer" 0 "(bIgnoreAllPressedKeysUntilRelease=True,bForceImmediately=False,bNotifyUserSettings=False)")
      (bind _asgm_main_game_mode (Utilities|Casting|CastToGM_MainGameMode (Game|GetGameMode)))
      (bind _output_get (Variables|Default|SetGameMode _asgm_main_game_mode))
      (Default|InitialiseGame _output_get (Game|Player|GetOwningPlayerController (Variables|Default|GetPlayerCameraManager))))))

(event Input|KeyboardEvents|O
  (params (Key :type Key%20Structure :default "None"))
  ;[1 1 1 1 58] Temporary Inputs
  (:Pressed
    (bind _asgm_main_game_mode (Utilities|Casting|CastToGM_MainGameMode (Game|GetGameMode)))
    (Default|StartRaffle _asgm_main_game_mode self)))

(event Input|KeyboardEvents|P
  (params (Key :type Key%20Structure :default "None"))
  ;[1 1 1 1 58] Temporary Inputs
  (:Pressed
    (Default|TogglePlayerIcons (Variables|Default|GetGameMode))))

(event Input|KeyboardEvents|Right
  (params (Key :type Key%20Structure :default "None"))
  (bind _gamemode (Variables|Default|GetGameMode))
  (bind _gamemode_2 (Variables|Default|GetGameMode))
  ;[1 0.8128 0 1 34] Control Player Cycling For Testing
  ;;[1 1 1] Cycle Player To The Right
  (:Pressed
    (bind _output_get (Variables|/Game/GM_MainGameMode.GM_MainGameMode_C|SetSelectedPlayer _gamemode_2 (+ (Variables|/Game/GM_MainGameMode.GM_MainGameMode_C|GetSelectedPlayer _gamemode) 1)))
    (if (>= _output_get (Utilities|Array|Length (Variables|/Game/GM_MainGameMode.GM_MainGameMode_C|GetExamplePlayers _gamemode)))
      (Variables|/Game/GM_MainGameMode.GM_MainGameMode_C|SetSelectedPlayer _gamemode_2 0))
    (Default|UpdateCurrentPlayer _gamemode_2)))

(event Input|KeyboardEvents|Left
  (params (Key :type Key%20Structure :default "None"))
  (bind _gamemode (Variables|Default|GetGameMode))
  (bind _gamemode_2 (Variables|Default|GetGameMode))
  ;[1 0.8128 0 1 34] Control Player Cycling For Testing
  ;;[1 1 1] Cycle Players To The Left
  (:Pressed
    (bind _output_get (Variables|/Game/GM_MainGameMode.GM_MainGameMode_C|SetSelectedPlayer _gamemode (- (Variables|/Game/GM_MainGameMode.GM_MainGameMode_C|GetSelectedPlayer _gamemode_2) 1)))
    (if (< _output_get 0)
      (Variables|/Game/GM_MainGameMode.GM_MainGameMode_C|SetSelectedPlayer _gamemode (- (Utilities|Array|Length (Variables|/Game/GM_MainGameMode.GM_MainGameMode_C|GetExamplePlayers _gamemode_2)) 1)))
    (Default|UpdateCurrentPlayer _gamemode)))

(fn ConstructionScript)