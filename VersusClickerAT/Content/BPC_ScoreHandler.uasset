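; Score component that grows one player's raffle score over time, addressing that player by ID in GM_MainGameMode's ExamplePlayers array.
; Shortly after BeginPlay, it fills UpgradeValues from the "Upgrade0" row of each ScoreManager upgrade table.
; StartCalculation starts two looping timers, lag and auto-click, at different intervals.
; Both currently apply identical logic, adding ScoreAddition to Score for participating players, without using UpgradeValues.
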(event Custom|UpdateLagScore
  ;[0.6911 1 0.2028 1 34] Add Score increment to player score, if the player is participating in the raffle
  (bind _asgm_main_game_mode (Utilities|Casting|CastToGM_MainGameMode (Game|GetGameMode)))
  (if (.participating (Utilities|Array|Get(acopy) (Variables|/Game/GM_MainGameMode.GM_MainGameMode_C|GetExamplePlayers _asgm_main_game_mode) (Variables|Default|GetID)))
    (Utilities|Array|SetArrayElem (Variables|/Game/GM_MainGameMode.GM_MainGameMode_C|GetExamplePlayers _asgm_main_game_mode) (.id (Utilities|Array|Get(acopy) (Variables|/Game/GM_MainGameMode.GM_MainGameMode_C|GetExamplePlayers _asgm_main_game_mode) (Variables|Default|GetID))) (Utilities|Struct|MakeSTRUCT_Viewer (.username (Utilities|Array|Get(acopy) (Variables|/Game/GM_MainGameMode.GM_MainGameMode_C|GetExamplePlayers _asgm_main_game_mode) (Variables|Default|GetID))) (.profilepicture (Utilities|Array|Get(acopy) (Variables|/Game/GM_MainGameMode.GM_MainGameMode_C|GetExamplePlayers _asgm_main_game_mode) (Variables|Default|GetID))) (.id (Utilities|Array|Get(acopy) (Variables|/Game/GM_MainGameMode.GM_MainGameMode_C|GetExamplePlayers _asgm_main_game_mode) (Variables|Default|GetID))) (+ (.score (Utilities|Array|Get(acopy) (Variables|/Game/GM_MainGameMode.GM_MainGameMode_C|GetExamplePlayers _asgm_main_game_mode) (Variables|Default|GetID))) (.scoreaddition (Utilities|Array|Get(acopy) (Variables|/Game/GM_MainGameMode.GM_MainGameMode_C|GetExamplePlayers _asgm_main_game_mode) (Variables|Default|GetID)))) (.scoreaddition (Utilities|Array|Get(acopy) (Variables|/Game/GM_MainGameMode.GM_MainGameMode_C|GetExamplePlayers _asgm_main_game_mode) (Variables|Default|GetID))) (.participating (Utilities|Array|Get(acopy) (Variables|/Game/GM_MainGameMode.GM_MainGameMode_C|GetExamplePlayers _asgm_main_game_mode) (Variables|Default|GetID))) (.scorecalculator (Utilities|Array|Get(acopy) (Variables|/Game/GM_MainGameMode.GM_MainGameMode_C|GetExamplePlayers _asgm_main_game_mode) (Variables|Default|GetID)))))))

(event Custom|UpdateAutoClickScore
  ;[0.6911 1 0.2028 1 34] Add Score increment to player score, if the player is participating in the raffle
  (bind _asgm_main_game_mode (Utilities|Casting|CastToGM_MainGameMode (Game|GetGameMode)))
  (if (.participating (Utilities|Array|Get(acopy) (Variables|/Game/GM_MainGameMode.GM_MainGameMode_C|GetExamplePlayers _asgm_main_game_mode) (Variables|Default|GetID)))
    (Utilities|Array|SetArrayElem (Variables|/Game/GM_MainGameMode.GM_MainGameMode_C|GetExamplePlayers _asgm_main_game_mode) (.id (Utilities|Array|Get(acopy) (Variables|/Game/GM_MainGameMode.GM_MainGameMode_C|GetExamplePlayers _asgm_main_game_mode) (Variables|Default|GetID))) (Utilities|Struct|MakeSTRUCT_Viewer (.username (Utilities|Array|Get(acopy) (Variables|/Game/GM_MainGameMode.GM_MainGameMode_C|GetExamplePlayers _asgm_main_game_mode) (Variables|Default|GetID))) (.profilepicture (Utilities|Array|Get(acopy) (Variables|/Game/GM_MainGameMode.GM_MainGameMode_C|GetExamplePlayers _asgm_main_game_mode) (Variables|Default|GetID))) (.id (Utilities|Array|Get(acopy) (Variables|/Game/GM_MainGameMode.GM_MainGameMode_C|GetExamplePlayers _asgm_main_game_mode) (Variables|Default|GetID))) (+ (.score (Utilities|Array|Get(acopy) (Variables|/Game/GM_MainGameMode.GM_MainGameMode_C|GetExamplePlayers _asgm_main_game_mode) (Variables|Default|GetID))) (.scoreaddition (Utilities|Array|Get(acopy) (Variables|/Game/GM_MainGameMode.GM_MainGameMode_C|GetExamplePlayers _asgm_main_game_mode) (Variables|Default|GetID)))) (.scoreaddition (Utilities|Array|Get(acopy) (Variables|/Game/GM_MainGameMode.GM_MainGameMode_C|GetExamplePlayers _asgm_main_game_mode) (Variables|Default|GetID))) (.participating (Utilities|Array|Get(acopy) (Variables|/Game/GM_MainGameMode.GM_MainGameMode_C|GetExamplePlayers _asgm_main_game_mode) (Variables|Default|GetID))) (.scorecalculator (Utilities|Array|Get(acopy) (Variables|/Game/GM_MainGameMode.GM_MainGameMode_C|GetExamplePlayers _asgm_main_game_mode) (Variables|Default|GetID)))))))

(event Custom|StartCalculation
  ;[1 1 1] Sets up the score increment function to happen on a timer (15 IS DEFAULT)
  (Utilities|Casting|CastToGM_MainGameMode (Game|GetGameMode))
  ;;[1 0.2247 0.991] LAG SCORE
  (Utilities|Time|SetTimerbyFunctionName 0 "UpdateLagScore" 5.0 true)
  ;;[1 0.2247 0.991] AUTO CLICK SCORE
  (Utilities|Time|SetTimerbyFunctionName 0 "UpdateAutoClickScore" 8.0 true))

(event EventBeginPlay
  (Utilities|FlowControl|Delay 0.2)
  (bind _asgm_main_game_mode (Utilities|Casting|CastToGM_MainGameMode (Game|GetGameMode)))
  (for (_array_element _array_index) (Variables|/Game/BP_ScoreManager.BP_ScoreManager_C|GetUpgradeCurves (Variables|/Game/GM_MainGameMode.GM_MainGameMode_C|GetScoreManager _asgm_main_game_mode))
    (bind _returnvalue (Utilities|GetDataTableRow _array_element (Utilities|String|StringToName (Utilities|String|MakeLiteralString "Upgrade0")))
      (:then
        (Utilities|Array|SetArrayElem (Variables|Default|GetUpgradeValues) _array_index (Utilities|Struct|BreakSTRUCT_UpgradeCurve _returnvalue))))))