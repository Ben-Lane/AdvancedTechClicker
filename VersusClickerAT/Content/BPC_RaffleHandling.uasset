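; Game mode component that runs the raffle timer countdown on behalf of the streamer HUD's raffle widget.
; ContinueRaffleCountdown copies the shrink rate and timer bar width from the widget, then Tick reduces that width without touching the UI.
; StopRaffleCountdown halts the calculation, writes the width back to the bar and returns the widget.
; When the width runs out, UpdateRaffleWidget does the same stop and calls TimerHasEnded on the widget.
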(event EventTick
  (params (DeltaSeconds :type Float%20%28single-precision%29))
  (if (Variables|Default|GetHandleCalculations)
    (bind _output_get (Variables|Default|SetTimerWidth (- (Variables|Default|GetTimerWidth) (* (Variables|Default|GetShrinkPerSec) DeltaSeconds))))
    (if (<= _output_get 0.0)
      (CallFunction|UpdateRaffleWidget))))

(fn ContinueRaffleCountdown
  (bind _asgm_main_game_mode (Utilities|Casting|CastToGM_MainGameMode (Components|GetOwner self)))
  (Variables|Default|SetShrinkPerSec (Variables|/Game/UI/ViewerExclusive/WB_Raffle.WB_Raffle_C|GetShrinkPerSec (Variables|/Game/UI/GeneralUI/WB_StreamerHUD.WB_StreamerHUD_C|GetWB_Raffle (Variables|/Game/UI/ViewerExclusive/WB_ViewerHUD.WB_ViewerHUD_C|GetWB_StreamerHUD (Variables|/Game/UI/ViewerExclusive/WB_ViewerPerspective.WB_ViewerPerspective_C|GetWB_ViewerHUD (Variables|/Game/GM_MainGameMode.GM_MainGameMode_C|GetViewerHUD _asgm_main_game_mode))))))
  (Variables|Default|SetTimerWidth (.x (Class|Widget|GetDesiredSize (Variables|/Game/UI/ViewerExclusive/WB_Raffle.WB_Raffle_C|GetTimerBar (Variables|/Game/UI/GeneralUI/WB_StreamerHUD.WB_StreamerHUD_C|GetWB_Raffle (Variables|/Game/UI/ViewerExclusive/WB_ViewerHUD.WB_ViewerHUD_C|GetWB_StreamerHUD (Variables|/Game/UI/ViewerExclusive/WB_ViewerPerspective.WB_ViewerPerspective_C|GetWB_ViewerHUD (Variables|/Game/GM_MainGameMode.GM_MainGameMode_C|GetViewerHUD _asgm_main_game_mode))))))))
  (Variables|Default|SetHandleCalculations true))

(fn StopRaffleCountdown
  (Variables|Default|SetHandleCalculations false)
  (bind _asgm_main_game_mode (Utilities|Casting|CastToGM_MainGameMode (Components|GetOwner self)))
  (Class|Image|SetDesiredSizeOverride (Variables|/Game/UI/ViewerExclusive/WB_Raffle.WB_Raffle_C|GetTimerBar (Variables|/Game/UI/GeneralUI/WB_StreamerHUD.WB_StreamerHUD_C|GetWB_Raffle (Variables|/Game/UI/ViewerExclusive/WB_ViewerHUD.WB_ViewerHUD_C|GetWB_StreamerHUD (Variables|/Game/UI/ViewerExclusive/WB_ViewerPerspective.WB_ViewerPerspective_C|GetWB_ViewerHUD (Variables|/Game/GM_MainGameMode.GM_MainGameMode_C|GetViewerHUD _asgm_main_game_mode))))) (Math|Vector2D|MakeVector2D (Variables|Default|GetTimerWidth) (.y (Class|Widget|GetDesiredSize (Variables|/Game/UI/ViewerExclusive/WB_Raffle.WB_Raffle_C|GetTimerBar (Variables|/Game/UI/GeneralUI/WB_StreamerHUD.WB_StreamerHUD_C|GetWB_Raffle (Variables|/Game/UI/ViewerExclusive/WB_ViewerHUD.WB_ViewerHUD_C|GetWB_StreamerHUD (Variables|/Game/UI/ViewerExclusive/WB_ViewerPerspective.WB_ViewerPerspective_C|GetWB_ViewerHUD (Variables|/Game/GM_MainGameMode.GM_MainGameMode_C|GetViewerHUD _asgm_main_game_mode)))))))))
  (return (Variables|/Game/UI/GeneralUI/WB_StreamerHUD.WB_StreamerHUD_C|GetWB_Raffle (Variables|/Game/UI/ViewerExclusive/WB_ViewerHUD.WB_ViewerHUD_C|GetWB_StreamerHUD (Variables|/Game/UI/ViewerExclusive/WB_ViewerPerspective.WB_ViewerPerspective_C|GetWB_ViewerHUD (Variables|/Game/GM_MainGameMode.GM_MainGameMode_C|GetViewerHUD _asgm_main_game_mode))))))

(fn UpdateRaffleWidget
  (bind _wb_raffle (CallFunction|StopRaffleCountdown))
  (Default|TimerHasEnded _wb_raffle))