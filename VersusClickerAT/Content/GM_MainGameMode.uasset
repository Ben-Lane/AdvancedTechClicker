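; Game mode for a streamer/viewer interaction demo that switches between streamer and viewer perspectives and runs viewer raffles.
; InitialiseGame creates both HUD widgets and fills a profile-picture icon bar from example players, highlighting the selected one.
; StartRaffle sets the event state and shows the raffle widget, while EnterRaffle adds the selected player unless already entered.
; A FlipFlop toggles viewer HUD visibility, resuming the raffle component's countdown only in streamer view.
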(event Custom|TogglePerspective
  (bind _viewerhud (Variables|Default|GetViewerHUD))
  (bind _currentevent (Variables|Default|GetCurrentEvent))
  (bind _bpc_rafflehandling (Variables|Default|GetBPC_RaffleHandling))
  (bind _returnvalue (Utilities|Enum|Equal(Enum) _currentevent "NewEnumerator1"))
  ;[1 1 1] Toggles between streamer and viewer view
  (Utilities|FlowControl|FlipFlop
    (:A
      (Variables|Default|SetStreamerPerspective true)
      (Variables|/Script/UMG.Widget|SetVisibility _viewerhud "Hidden")
      ;;[0.492 1 0] If a raffle is currently active
      (if _returnvalue
        (Default|ContinueRaffleCountdown _bpc_rafflehandling)))
    (:B
      (Variables|Default|SetStreamerPerspective false)
      (Variables|/Script/UMG.Widget|SetVisibility _viewerhud "Visible")
      (if _returnvalue
        (Default|StopRaffleCountdown _bpc_rafflehandling)))))

(event EventBeginPlay
  (Variables|Default|SetCurrentEvent "NewEnumerator0"))

(event EventTick
  (params (DeltaSeconds :type Float%20%28single-precision%29)))

(fn ConstructionScript)

(fn StartRaffle
  (params (Host :type BP%20Main%20Player%20Controller%20Object%20Reference))
  (bind _viewerhud (Variables|Default|GetViewerHUD))
  (bind _wb_viewerhud (Variables|/Game/UI/ViewerExclusive/WB_ViewerPerspective.WB_ViewerPerspective_C|GetWB_ViewerHUD _viewerhud))
  (bind _wb_raffle (Variables|/Game/UI/ViewerExclusive/WB_ViewerHUD.WB_ViewerHUD_C|GetWB_Raffle _wb_viewerhud))
  ;[1 1 1 1 26] If a raffle doesnt already exist, one will be made, changing the state of this blueprint to say so
  (if (Utilities|Enum|NotEqual(Enum) (Variables|Default|GetCurrentEvent) "NewEnumerator1")
    (Variables|Default|SetCurrentEvent "NewEnumerator1")
    (Development|PrintString "Raffle Started")
    (Default|StartRaffle _wb_raffle)
    (Variables|/Script/UMG.Widget|SetVisibility _wb_raffle "Visible")
    (if (Utilities|Enum|NotEqual(Enum) (Variables|/Script/UMG.Widget|GetVisibility (Variables|Default|GetViewerHUD)) "Visible")
      (Default|ContinueRaffleCountdown (Variables|Default|GetBPC_RaffleHandling)))))

(fn EnterRaffle
  (bind _viewerhud (Variables|Default|GetViewerHUD))
  (bind _wb_viewerhud (Variables|/Game/UI/ViewerExclusive/WB_ViewerPerspective.WB_ViewerPerspective_C|GetWB_ViewerHUD _viewerhud))
  (bind _wb_raffle (Variables|/Game/UI/ViewerExclusive/WB_ViewerHUD.WB_ViewerHUD_C|GetWB_Raffle _wb_viewerhud))
  (LocalVariables|SetPlayerAlreadyEntered false)
  ;[1 1 1] Has Viewer already entered the raffle
  (bind _array_element (Utilities|Array|ForEachLoopwithBreak (Variables|/Game/UI/ViewerExclusive/WB_Raffle.WB_Raffle_C|GetRaffleEntries (Variables|/Game/UI/ViewerExclusive/WB_ViewerHUD.WB_ViewerHUD_C|GetWB_Raffle (Variables|/Game/UI/ViewerExclusive/WB_ViewerPerspective.WB_ViewerPerspective_C|GetWB_ViewerHUD (Variables|Default|GetViewerHUD)))) :!label _label)
    (:LoopBody
      (if (== (Variables|Default|GetSelectedPlayer) (.ID (Utilities|Struct|BreakSTRUCT_Viewer _array_element)))
        (LocalVariables|SetPlayerAlreadyEntered true)
        (goto _label Break)))
    (:Completed
      (if (not (LocalVariables|GetPlayerAlreadyEntered))
        ;[1 1 1] If not, Add To Raffle
        (Utilities|Array|Add (Variables|/Game/UI/ViewerExclusive/WB_Raffle.WB_Raffle_C|GetRaffleEntries _wb_raffle) (Utilities|Array|Get(acopy) (Variables|Default|GetExamplePlayers) (Variables|Default|GetSelectedPlayer)))
        (Default|PlayerEntered _wb_raffle)
        (else
          (Development|PrintString "Not Added To Raffle ")))
      (return (not (LocalVariables|GetPlayerAlreadyEntered))))))

(fn InitialiseGame
  (params (Player :type Player%20Controller%20Object%20Reference))
  ;[1 0.2244 0 1 26] This creates all widgets that will be default in the project, as well as any setup needed.
  (bind _output_get (Variables|Default|SetController Player))
  (bind _returnvalue (UserInterface|CreateWidget "/Game/UI/GeneralUI/WB_StreamerHUD.WB_StreamerHUD_C" _output_get self))
  (bind _output_get_2 (Variables|Default|SetStreamerHUD _returnvalue))
  (UserInterface|Viewport|AddtoPlayerScreen _output_get_2)
  (bind _returnvalue_2 (UserInterface|CreateWidget "/Game/UI/ViewerExclusive/WB_ViewerPerspective.WB_ViewerPerspective_C" Player self))
  (bind _output_get_3 (Variables|Default|SetViewerHUD _returnvalue_2))
  (UserInterface|Viewport|AddtoPlayerScreen _output_get_3)
  (Variables|/Script/Engine.PlayerController|SetbShowMouseCursor Player true)
  (CallFunction|CreatePlayerIcons))

(fn CreatePlayerIcons
  ;[1 1 1 1 25] If the player icons have not been generated, it will create the visual to represent the current player selected, using player structures to obtain their player profile picture
  (for _array_element (Variables|Default|GetExamplePlayers)
    (Default|AddImages (Variables|/Game/UI/ViewerExclusive/WB_ViewerPerspective.WB_ViewerPerspective_C|GetPlayerIconsBox (Variables|Default|GetViewerHUD)) (Variables|Default|GetController) (.profilepicture _array_element)))
  (CallFunction|UpdateCurrentPlayer))

(fn UpdateCurrentPlayer
  ;[1 1 1] Find currently selected user
  (for (_array_element _array_index) (Class|PanelWidget|GetAllChildren (Variables|/Game/UI/GeneralUI/WB_PlayerIconDisplay.WB_PlayerIconDisplay_C|GetPictureLine (Variables|/Game/UI/ViewerExclusive/WB_ViewerPerspective.WB_ViewerPerspective_C|GetPlayerIconsBox (Variables|Default|GetViewerHUD))))
    (bind _aswb_icon (Utilities|Casting|CastToWB_Icon _array_element))
    (if (!= _array_index (Variables|Default|GetSelectedPlayer))
      ;[1 1 1] Change Selected User Background To Unselected
      (Default|UpdateOutline _aswb_icon (Math|Conversions|ToColor(LinearColor) (Class|KismetMathLibrary|LinearColorWhite)))
      (else
        ;[1 1 1] Change User Selected Background To Selected
        (Default|UpdateOutline _aswb_icon (Math|Conversions|ToColor(LinearColor) (Class|KismetMathLibrary|LinearColorBlue)))))))